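; BP_BasicEnemy is a basic enemy with health, a red world-space health bar widget, and death handling.
; Each tick the health bar rotates to face the player camera.
; UpdateHealthBar subtracts incoming damage on a hit and updates the bar's percent and displayed status.
; At zero health or below, the enemy destroys itself and asks its CombatZone to check whether combat has ended.
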(event Custom|UpdateHealthBar
  (params (HitReceived :type Boolean) (DamageReceived :type Integer))
  ;[1 1 1] Health bar update
  (if HitReceived
    (Variables|Default|SetHealth (- (Variables|Default|GetHealth) DamageReceived))
    (bind _aswb_health_bar (Utilities|Casting|CastToWB_HealthBar (UserInterface|GetWidget (Variables|Default|GetHealthBar))))
    (Progress|SetPercent (Variables|/Game/Blueprints/AI/WB_HealthBar.WB_HealthBar_C|GetHealthBar _aswb_health_bar) (/ (Variables|Default|GetHealth) (Variables|Default|GetMax_Health)))
    (Variables|/Game/Blueprints/AI/WB_HealthBar.WB_HealthBar_C|SetStatus_Displayed _aswb_health_bar (Variables|Default|GetStatus))
    (if (<= (Variables|Default|GetHealth) 0.0)
      (Actor|DestroyActor)
      (Default|CombatEndCheck (Variables|Default|GetCombatZone)))))

(event EventBeginPlay
  (bind _healthbar (Variables|Default|GetHealthBar))
  (bind _aswb_health_bar (Utilities|Casting|CastToWB_HealthBar (UserInterface|GetWidget _healthbar)))
  (Variables|/Script/UMG.ProgressBar|SetFillColorAndOpacity (Variables|/Game/Blueprints/AI/WB_HealthBar.WB_HealthBar_C|GetHealthBar _aswb_health_bar) "(R=1.000000,G=0.000000,B=0.000000,A=1.000000)")
  (Rendering|SetCastShadow _healthbar false)
  (Variables|Default|SetHealth (Variables|Default|GetMax_Health)))

(event EventTick
  (params (DeltaSeconds :type Float%20%28single-precision%29))
  (bind _healthbar (Variables|Default|GetHealthBar))
  ;[1 1 1] Widget update
  (Transformation|SetWorldRotation _healthbar (Math|Rotator|FindLookatRotation (Transformation|GetWorldLocation _healthbar) (Transformation|GetWorldLocation (Variables|/Script/Engine.PlayerCameraManager|GetTransformComponent (Game|GetPlayerCameraManager 0)))) false false))

(fn ConstructionScript)