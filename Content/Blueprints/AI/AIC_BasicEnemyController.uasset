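; AI controller for BP_BasicEnemy in turn-based, grid-based combat, running the BT_BasicEnemy behavior tree.
; Combat events write combat state, turn count and current turn to the Blackboard, marking the turn active when it matches this enemy's position in the combatant list.
; On its turn the enemy turns red and applies its status: Burning deals damage scaled by the player's FireLevel, while Frozen and Shocked set Blackboard flags.
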(event Custom|Update%20Combat%20Status
  (AI|Components|Blackboard|SetValueasBool (AI|GetBlackboard 0) (Variables|Default|GetBlackboardCombatBoolKeyName) true)
  (Variables|Default|SetIsEnemyInCombat true))

(event EventBeginPlay
  (AI|RunBehaviorTree "/Game/Blueprints/AI/BT_BasicEnemy.BT_BasicEnemy")
  (Utilities|Casting|CastToBP_TopDownGameMode (Game|GetGameMode))
  (Input|EnableInput (Game|GetPlayerController 0))
  (bind _asbp_top_down_controller (Utilities|Casting|CastToBP_TopDownController (Game|GetPlayerController 0)))
  (Variables|Default|SetPlayerControllerRef _asbp_top_down_controller))

(event EventTick
  (params (DeltaSeconds :type Float%20%28single-precision%29)))

(event EventPossess
  (params (PossessedPawn :type Pawn%20Object%20Reference))
  (bind _asbp_basic_enemy (Utilities|Casting|CastToBP_BasicEnemy PossessedPawn))
  (bind _output_get (Variables|Default|SetPawnRef _asbp_basic_enemy))
  (Variables|Default|SetGridRef (Variables|/Game/Blueprints/AI/BP_BasicEnemy.BP_BasicEnemy_C|GetGridRef _output_get)))

(event EventUpdateEnemiesInsideCombat
  (params (Enemies :type Array%20of%20BP%20Basic%20Enemy%20Object%20References))
  (for (_array_element _array_index) Enemies
    (if (== _array_element (Variables|Default|GetPawnRef))
      (Variables|Default|SetEnemyCombatIndex (+ _array_index 1))))
  (for _array_element_2 Enemies
    (Class|BlackboardComponent|SetValueasInt (AI|GetBlackboard 0) (Variables|Default|GetMaxTurnIndexBlackboardKey) (Utilities|Array|Length Enemies))))

(event EventChangeTurnIndex
  (params (TurnIndex :type Integer))
  (bind _returnvalue (AI|GetBlackboard 0))
  (bind _returnvalue_2 (AI|GetBlackboard 0))
  (bind _returnvalue_3 (AI|GetBlackboard 0))
  (bind _pawnref (Variables|Default|GetPawnRef))
  (bind _pawnref_2 (Variables|Default|GetPawnRef))
  (bind _enemycombatindex (Variables|Default|GetEnemyCombatIndex))
  (bind _returnvalue_4 (== TurnIndex _enemycombatindex))
  (bind _mesh (Variables|/Script/Engine.Character|GetMesh _pawnref))
  (Class|BlackboardComponent|SetValueasInt (AI|GetBlackboard 0) (Variables|Default|GetBlackboardTurnIndexKeyName) TurnIndex)
  (AI|Components|Blackboard|SetValueasBool (AI|GetBlackboard 0) (Variables|Default|GetBlackboardActiveTurnKeyName) _returnvalue_4)
  (if _returnvalue_4
    (Rendering|Material|SetMaterial _mesh 0 "/Game/Characters/Mannequins/Materials/Instances/Manny/MI_Manny_02_Red.MI_Manny_02_Red")
    (Rendering|Material|SetMaterial _mesh 1 "/Game/Characters/Mannequins/Materials/Instances/Manny/MI_Manny_01_Red.MI_Manny_01_Red")
    (switch Utilities|FlowControl|Switch|SwitchonE_Status (Variables|/Game/Blueprints/AI/BP_BasicEnemy.BP_BasicEnemy_C|GetStatus _pawnref_2)
      (:NewEnumerator1
        (AI|Components|Blackboard|SetValueasBool _returnvalue (Variables|Default|GetIsFrozenBlackboardKey) false)
        (AI|Components|Blackboard|SetValueasBool _returnvalue (Variables|Default|GetIsShockedBlackboardKey) false)
        (Default|UpdateHealthBar _pawnref_2 true (Math|Float|Truncate (* (Variables|/Game/TopDown/Blueprints/BP_TopDownController.BP_TopDownController_C|GetFireLevel (Variables|Default|GetPlayerControllerRef)) 5))))
      (:NewEnumerator2
        (AI|Components|Blackboard|SetValueasBool _returnvalue_2 (Variables|Default|GetIsShockedBlackboardKey) false)
        (AI|Components|Blackboard|SetValueasBool _returnvalue_2 (Variables|Default|GetIsFrozenBlackboardKey) true))
      (:NewEnumerator3
        (AI|Components|Blackboard|SetValueasBool _returnvalue_3 (Variables|Default|GetIsFrozenBlackboardKey) false)
        (AI|Components|Blackboard|SetValueasBool _returnvalue_3 (Variables|Default|GetIsShockedBlackboardKey) true)))
    (else
      (Rendering|Material|SetMaterial _mesh 0 "/Game/Characters/Mannequins/Materials/Instances/Manny/MI_Manny_02.MI_Manny_02")
      (Rendering|Material|SetMaterial _mesh 1 "/Game/Characters/Mannequins/Materials/Instances/Manny/MI_Manny_01.MI_Manny_01"))))

(fn ConstructionScript)

(fn GetPositiononGrid
  (params (ActorOnGrid :type Actor%20Object%20Reference))
  (bind (_isvalid _row _column) (Default|LocationtoTile (Variables|Default|GetGridRef) (Transformation|GetActorLocation)))
  (return (Math|Vector2D|MakeVector2D (Math|Conversions|ToFloat(Integer) _row) (Math|Conversions|ToFloat(Integer) _column))))