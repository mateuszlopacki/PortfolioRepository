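; BP_Heal is an interactable pickup that restores the player character's health.
; The IA_Interact input only takes effect while the WidgetTimerHandle timer is active, so that timer acts as the interaction gate.
; It then sets BP_TopDownCharacter's Health to full, refreshes the health bar and destroys itself.
; The construction script runs the parent's, then passes ParticleColor to the interactable Niagara effect.
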(event Input|EnhancedActionEvents|EnhancedInputActionIA_Interact
  (params (ActionValue :type Boolean) (ElapsedSeconds :type Float%20%28double-precision%29) (TriggeredSeconds :type Float%20%28double-precision%29) (InputAction :type Input%20Action%20Object%20Reference :default "/Game/TopDown/Input/Actions/IA_Interact.IA_Interact"))
  (:Started
    (if (Utilities|Time|IsTimerActivebyHandle (Variables|Default|GetWidgetTimerHandle))
      (bind _asbp_top_down_character (Utilities|Casting|CastToBP_TopDownCharacter (Game|GetPlayerCharacter 0)))
      (Variables|/Game/TopDown/Blueprints/BP_TopDownCharacter.BP_TopDownCharacter_C|SetHealth _asbp_top_down_character 1e+02)
      (Default|UpdateHealthBar _asbp_top_down_character 0.0)
      (Actor|DestroyActor))))

(event EventBeginPlay
  (|CallParentFunction) ; This node is disabled and will not be called.\nDrag off pins to build functionality.
)

(event Collision|EventActorBeginOverlap
  (params (OtherActor :type Actor%20Object%20Reference))
  (|CallParentFunction OtherActor) ; This node is disabled and will not be called.\nDrag off pins to build functionality.
)

(event EventTick
  (params (DeltaSeconds :type Float%20%28single-precision%29)))

(fn ConstructionScript
  (|CallParentFunction)
  (Niagara|SetNiagaraVariable(LinearColor) (Variables|Default|GetNS_InteractablesEffect) "ParticleColor" (Variables|Default|GetParticleColor)))