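; Interactable pickup that permanently upgrades the player's maximum action and movement points.
; On Interact input, while the widget timer is active, it raises both maximums on BP_TopDownController by one and destroys itself.
; It then shows a congratulations message through the CombatHUD text popup and sets the controller to ignore move input.
; The widget timer is only checked here, never started.
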(event Input|EnhancedActionEvents|EnhancedInputActionIA_Interact
  (params (ActionValue :type Boolean) (ElapsedSeconds :type Float%20%28double-precision%29) (TriggeredSeconds :type Float%20%28double-precision%29) (InputAction :type Input%20Action%20Object%20Reference :default "/Game/TopDown/Input/Actions/IA_Interact.IA_Interact"))
  (:Started
    (if (Utilities|Time|IsTimerActivebyHandle (Variables|Default|GetWidgetTimerHandle))
      (bind _asbp_top_down_controller (Utilities|Casting|CastToBP_TopDownController (Game|GetPlayerController 0)))
      (Variables|/Game/TopDown/Blueprints/BP_TopDownController.BP_TopDownController_C|SetMax_MovementPoints _asbp_top_down_controller (+ (Variables|/Game/TopDown/Blueprints/BP_TopDownController.BP_TopDownController_C|GetMax_MovementPoints _asbp_top_down_controller) 1))
      (Variables|/Game/TopDown/Blueprints/BP_TopDownController.BP_TopDownController_C|SetMax_ActionPoints _asbp_top_down_controller (+ (Variables|/Game/TopDown/Blueprints/BP_TopDownController.BP_TopDownController_C|GetMax_ActionPoints _asbp_top_down_controller) 1))
      (Actor|DestroyActor)
      (bind _ascombat_hud (Utilities|Casting|CastToCombatHUD (HUD|GetHUD (Game|GetPlayerController 0))))
      (Variables|/Game/HUDs/WB_TextPopup.WB_TextPopup_C|SetDisplayedText (Variables|/Game/HUDs/CombatHUD.CombatHUD_C|GetTextPopup_Ref _ascombat_hud) "Congratulations, you've found a powerful upgrade! 
 
Your Action and Movement points have been increased by 1!")
      (Widget|SetVisibility (Variables|/Game/HUDs/CombatHUD.CombatHUD_C|GetTextPopup_Ref _ascombat_hud) "SelfHitTestInvisible")
      (bind _asbp_top_down_controller_2 (Utilities|Casting|CastToBP_TopDownController (Game|GetPlayerController 0)))
      (Input|SetIgnoreMoveInput _asbp_top_down_controller_2 true))))

(event EventBeginPlay
  (|CallParentFunction) ; This node is disabled and will not be called.\nDrag off pins to build functionality.
)

(event Collision|EventActorBeginOverlap
  (params (OtherActor :type Actor%20Object%20Reference))
  (|CallParentFunction OtherActor) ; This node is disabled and will not be called.\nDrag off pins to build functionality.
)

(event EventTick
  (params (DeltaSeconds :type Float%20%28single-precision%29)))

(fn ConstructionScript
  (|CallParentFunction))