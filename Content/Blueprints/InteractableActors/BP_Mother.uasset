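; BP_Mother is an interactable actor that triggers level sequences and reveals the combat skills button once its interaction has finished.
; When the close-popup input completes and InteractionFinished is set, a DoOnce gate creates a player for each entry in SequencesToPlay and starts them all in one loop.
; It then finds the first top-level WB_Combat widget and makes its SkillsButton visible.
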(event Input|EnhancedActionEvents|EnhancedInputActionIA_ClosePopup
  (params (ActionValue :type Boolean) (ElapsedSeconds :type Float%20%28double-precision%29) (TriggeredSeconds :type Float%20%28double-precision%29) (InputAction :type Input%20Action%20Object%20Reference :default "/Game/TopDown/Input/Actions/IA_ClosePopup.IA_ClosePopup"))
  (:Completed
    (if (Variables|Default|GetInteractionFinished)
      (Utilities|FlowControl|DoOnce false
        (:Completed
          (for _array_element (Variables|Default|GetSequencesToPlay)
            (bind _returnvalue (Sequencer|Player|CreateLevelSequencePlayer _array_element (Variables|Default|GetSettings)))
            (Sequencer|Player|Play _returnvalue :!class /Script/MovieScene.MovieSceneSequencePlayer))
          (bind _foundwidgets (Widget|GetAllWidgetsOfClass "/Game/HUDs/WB_Combat.WB_Combat_C" true))
          (Widget|SetVisibility (Variables|/Game/HUDs/WB_Combat.WB_Combat_C|GetSkills_Button (Utilities|Array|Get(acopy) _foundwidgets)) "Visible"))))))

(event EventBeginPlay
  (|CallParentFunction) ; This node is disabled and will not be called.\nDrag off pins to build functionality.
)

(event Collision|EventActorBeginOverlap
  (params (OtherActor :type Actor%20Object%20Reference))
  (|CallParentFunction OtherActor) ; This node is disabled and will not be called.\nDrag off pins to build functionality.
)

(event EventTick
  (params (DeltaSeconds :type Float%20%28single-precision%29)))

(fn ConstructionScript
  (|CallParentFunction))