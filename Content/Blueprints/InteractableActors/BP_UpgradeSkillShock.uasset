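; Interactable pickup that teaches or upgrades the player's Shock skill, then destroys itself.
; Interact input, accepted only while the widget timer is active, reads ShockLevel from the player controller and increments it.
; The first pickup enables the third HUD skill button; both cases show a text popup and block movement input.
; The construction script tints the Niagara effect and sets DisplayNote.
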(event Input|EnhancedActionEvents|EnhancedInputActionIA_Interact
  (params (ActionValue :type Boolean) (ElapsedSeconds :type Float%20%28double-precision%29) (TriggeredSeconds :type Float%20%28double-precision%29) (InputAction :type Input%20Action%20Object%20Reference :default "/Game/TopDown/Input/Actions/IA_Interact.IA_Interact"))
  (:Started
    (if (Utilities|Time|IsTimerActivebyHandle (Variables|Default|GetWidgetTimerHandle))
      (bind _asbp_top_down_controller (Utilities|Casting|CastToBP_TopDownController (Game|GetPlayerController 0)))
      (if (== (Variables|/Game/TopDown/Blueprints/BP_TopDownController.BP_TopDownController_C|GetShockLevel _asbp_top_down_controller) 0)
        (bind _ascombat_hud (Utilities|Casting|CastToCombatHUD (HUD|GetHUD _asbp_top_down_controller)))
        (Default|AddButtontoChangeState (Variables|/Game/HUDs/CombatHUD.CombatHUD_C|GetCombatHUD_Ref _ascombat_hud) (Variables|/Game/HUDs/WB_Combat.WB_Combat_C|GetSkill_3_Button (Variables|/Game/HUDs/CombatHUD.CombatHUD_C|GetCombatHUD_Ref _ascombat_hud)))
        (Class|Button|SetBackgroundColor (Variables|/Game/HUDs/WB_Combat.WB_Combat_C|GetSkill_3_Button (Variables|/Game/HUDs/CombatHUD.CombatHUD_C|GetCombatHUD_Ref _ascombat_hud)) "(R=1.000000,G=1.000000,B=1.000000,A=1.000000)")
        (Variables|/Game/HUDs/WB_TextPopup.WB_TextPopup_C|SetDisplayedText (Variables|/Game/HUDs/CombatHUD.CombatHUD_C|GetTextPopup_Ref _ascombat_hud) "You have just learned the power of lightnings! 
 
You have just acquired Shock skill. Shocked status prevents enemies from attacking - they can still move!")
        (Widget|SetVisibility (Variables|/Game/HUDs/CombatHUD.CombatHUD_C|GetTextPopup_Ref _ascombat_hud) "SelfHitTestInvisible")
        (else
          (bind _ascombat_hud_2 (Utilities|Casting|CastToCombatHUD (HUD|GetHUD _asbp_top_down_controller)))
          (Variables|/Game/HUDs/WB_TextPopup.WB_TextPopup_C|SetDisplayedText (Variables|/Game/HUDs/CombatHUD.CombatHUD_C|GetTextPopup_Ref _ascombat_hud_2) "Shock Skill upgraded! 
 
Your skill will deal more damage!")
          (Widget|SetVisibility (Variables|/Game/HUDs/CombatHUD.CombatHUD_C|GetTextPopup_Ref _ascombat_hud_2) "SelfHitTestInvisible")))
      (bind _asbp_top_down_controller_2 (Utilities|Casting|CastToBP_TopDownController (Game|GetPlayerController 0)))
      (Input|SetIgnoreMoveInput _asbp_top_down_controller_2 true)
      (Variables|/Game/TopDown/Blueprints/BP_TopDownController.BP_TopDownController_C|SetShockLevel _asbp_top_down_controller (+ (Variables|/Game/TopDown/Blueprints/BP_TopDownController.BP_TopDownController_C|GetShockLevel _asbp_top_down_controller) 1))
      (Actor|DestroyActor))))

(event EventBeginPlay
  (|CallParentFunction) ; This node is disabled and will not be called.\nDrag off pins to build functionality.
)

(event Collision|EventActorBeginOverlap
  (params (OtherActor :type Actor%20Object%20Reference))
  (|CallParentFunction OtherActor) ; This node is disabled and will not be called.\nDrag off pins to build functionality.
)

(event EventTick
  (params (DeltaSeconds :type Float%20%28single-precision%29)))

(fn ConstructionScript
  (|CallParentFunction)
  (Niagara|SetNiagaraVariable(LinearColor) (Variables|Default|GetNiagara) "ParticleColor" (Variables|Default|GetParticle%20Color))
  (Variables|Default|SetDisplayNote? true))