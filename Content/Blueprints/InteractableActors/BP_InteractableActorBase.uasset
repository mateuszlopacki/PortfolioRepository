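; Base interactable actor that shows a world-space prompt widget while the top-down character overlaps it and can open a text note.
; A looping timer turns the widget toward the camera, and its active handle doubles as the in-range check for interaction.
; If notes are enabled, interacting reveals the CombatHUD popup and ignores move input.
; The close-popup input then plays the configured level sequences once.
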(event Custom|AdjustWidgetPosition
  (bind _widget (Variables|Default|GetWidget))
  (Transformation|SetWorldRotation _widget (Math|Rotator|FindLookatRotation (Transformation|GetWorldLocation _widget) (Transformation|GetWorldLocation (Variables|/Script/Engine.PlayerCameraManager|GetTransformComponent (Game|GetPlayerCameraManager 0)))) false false))

(event Input|EnhancedActionEvents|EnhancedInputActionIA_Interact
  (params (ActionValue :type Boolean) (ElapsedSeconds :type Float%20%28double-precision%29) (TriggeredSeconds :type Float%20%28double-precision%29) (InputAction :type Input%20Action%20Object%20Reference :default "/Game/TopDown/Input/Actions/IA_Interact.IA_Interact"))
  (:Started
    (if (Utilities|Time|IsTimerActivebyHandle (Variables|Default|GetWidgetTimerHandle))
      (if (Variables|Default|GetDisplayNote?)
        (bind _ascombat_hud (Utilities|Casting|CastToCombatHUD (HUD|GetHUD (Game|GetPlayerController 0))))
        (Widget|SetVisibility (Variables|/Game/HUDs/CombatHUD.CombatHUD_C|GetTextPopup_Ref _ascombat_hud) "SelfHitTestInvisible")
        (Variables|Default|SetInteractionFinished true)
        (bind _asbp_top_down_controller (Utilities|Casting|CastToBP_TopDownController (Game|GetPlayerController 0)))
        (Input|SetIgnoreMoveInput _asbp_top_down_controller true)))))

(event Input|EnhancedActionEvents|EnhancedInputActionIA_ClosePopup
  (params (ActionValue :type Boolean) (ElapsedSeconds :type Float%20%28double-precision%29) (TriggeredSeconds :type Float%20%28double-precision%29) (InputAction :type Input%20Action%20Object%20Reference :default "/Game/TopDown/Input/Actions/IA_ClosePopup.IA_ClosePopup"))
  (:Completed
    (if (Variables|Default|GetInteractionFinished)
      (Utilities|FlowControl|DoOnce false
        (:Completed
          (for _array_element (Variables|Default|GetSequencesToPlay)
            (bind _returnvalue (Sequencer|Player|CreateLevelSequencePlayer _array_element (Variables|Default|GetSettings)))
            (Sequencer|Player|Play _returnvalue :!class /Script/MovieScene.MovieSceneSequencePlayer)))))))

(event EventBeginPlay
  (Rendering|SetCastShadow (Variables|Default|GetWidget) false)
  (Input|EnableInput (Game|GetPlayerController 0)))

(event Collision|EventActorBeginOverlap
  (params (OtherActor :type Actor%20Object%20Reference))
  (Utilities|Casting|CastToBP_TopDownCharacter OtherActor)
  (Development|SetHiddeninGame (Variables|Default|GetWidget) false false)
  (bind _ascombat_hud (Utilities|Casting|CastToCombatHUD (HUD|GetHUD (Game|GetPlayerController 0))))
  (Variables|/Game/HUDs/WB_TextPopup.WB_TextPopup_C|SetDisplayedText (Variables|/Game/HUDs/CombatHUD.CombatHUD_C|GetTextPopup_Ref _ascombat_hud) (Variables|Default|GetDisplayed%20Text))
  (bind _returnvalue (Utilities|Time|SetTimerbyEvent (delegate Custom|AdjustWidgetPosition) 0.05 true))
  (Variables|Default|SetWidgetTimerHandle _returnvalue))

(event Collision|EventActorEndOverlap
  (params (OtherActor :type Actor%20Object%20Reference))
  (Utilities|Casting|CastToBP_TopDownCharacter OtherActor)
  (Development|SetHiddeninGame (Variables|Default|GetWidget) true false)
  (Utilities|Time|ClearandInvalidateTimerbyHandle (Variables|Default|GetWidgetTimerHandle)))

(fn ConstructionScript)