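; Exploding barrel for grid-based combat that damages enemies and player characters on its four orthogonally adjacent tiles.
; Procedural meshes built from grid selection geometry mark those tiles, positioned and shown only while combat mode is enabled.
; Overlap with a BP_CheckingVolume at turn index 0 spawns probe volumes at the marked tiles to apply damage, then destroys the barrel.
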(event EventBeginPlay
  (bind _grid_ref (Variables|Default|GetGrid_Ref))
  (bind _materialinstance (CallFunction|CreateMaterialInstance (Variables|Default|GetDamageTilesColor) (Variables|Default|GetDamageTilesOpacity)))
  (Variables|Default|SetDamageTilesMaterial _materialinstance)
  (Class|ProceduralMeshComponent|CreateMeshSectionLinearColor (Variables|Default|GetProceduralMesh2) 0 (Variables|/Game/Blueprints/Grid/BP_Grid.BP_Grid_C|GetSelection%20Vertices _grid_ref) (Variables|/Game/Blueprints/Grid/BP_Grid.BP_Grid_C|GetSelection%20Triangles _grid_ref) 0 0 0 0 0 0 0 false false)
  (Rendering|Material|SetMaterial (Variables|Default|GetProceduralMesh2) 0 (Variables|Default|GetDamageTilesMaterial))
  (Rendering|SetVisibility (Variables|Default|GetProceduralMesh2) false false)
  (bind _asbp_top_down_controller (Utilities|Casting|CastToBP_TopDownController (Game|GetPlayerController 0)))
  (Variables|Default|SetPlayerControllerRef _asbp_top_down_controller))

(event EventTick
  (params (DeltaSeconds :type Float%20%28single-precision%29)))

(event EventUpdateCombatStatus
  (params (IsCombatModeEnabled :type Boolean) (IsMovementSelected :type Boolean) (IsSkillSelected :type Boolean))
  (bind _returnvalue (Transformation|GetActorLocation))
  (bind _grid_ref (Variables|Default|GetGrid_Ref))
  (bind _grid_ref_2 (Variables|Default|GetGrid_Ref))
  (bind _grid_ref_3 (Variables|Default|GetGrid_Ref))
  (bind _grid_ref_4 (Variables|Default|GetGrid_Ref))
  (if IsCombatModeEnabled
    (bind (_isvalid _row _column) (Default|LocationtoTile (Variables|Default|GetGrid_Ref) (Math|Vector|MakeVector (.x _returnvalue) (.y _returnvalue) (.z (Transformation|GetActorLocation (Variables|Default|GetGrid_Ref))))))
    (Utilities|FlowControl|Sequence
      (:then_0
        (bind _gridlocation (Default|TiletoGridLocation _grid_ref_4 (+ _row 1) (+ _column 0) false))
        (Transformation|SetWorldLocation (Variables|Default|GetProceduralMesh2) (Math|Conversions|ToVector(Vector2D) _gridlocation (+ (.z (Transformation|GetActorLocation _grid_ref_4)) -1.0)) false false))
      (:then_1
        (bind _gridlocation_2 (Default|TiletoGridLocation _grid_ref_2 (+ _row 0) (+ _column 1) false))
        (Transformation|SetWorldLocation (Variables|Default|GetProceduralMesh) (Math|Conversions|ToVector(Vector2D) _gridlocation_2 (+ (.z (Transformation|GetActorLocation _grid_ref_2)) -1.0)) false false))
      (:then_2
        (bind _gridlocation_3 (Default|TiletoGridLocation _grid_ref_3 (+ _row -1) (+ _column 0) false))
        (Transformation|SetWorldLocation (Variables|Default|GetProceduralMesh1) (Math|Conversions|ToVector(Vector2D) _gridlocation_3 (+ (.z (Transformation|GetActorLocation _grid_ref_3)) -1.0)) false false))
      (:then_3
        (bind _gridlocation_4 (Default|TiletoGridLocation _grid_ref (+ _row 0) (+ _column -1) false))
        (Transformation|SetWorldLocation (Variables|Default|GetProceduralMesh3) (Math|Conversions|ToVector(Vector2D) _gridlocation_4 (+ (.z (Transformation|GetActorLocation _grid_ref)) -1.0)) false false)
        (Rendering|SetVisibility (Variables|Default|GetProceduralMesh2) true false)))
    (else
      (Rendering|SetVisibility (Variables|Default|GetProceduralMesh2) false false))))

(event Collision|EventActorBeginOverlap
  (params (OtherActor :type Actor%20Object%20Reference))
  (Utilities|Casting|CastToBP_CheckingVolume OtherActor)
  (if (== (Variables|/Game/TopDown/Blueprints/BP_TopDownController.BP_TopDownController_C|GetTurnIndex (Variables|Default|GetPlayerControllerRef)) 0)
    (for _array_element (Utilities|Array|MakeArray (Variables|Default|GetProceduralMesh1) (Variables|Default|GetProceduralMesh2) (Variables|Default|GetProceduralMesh3) (Variables|Default|GetProceduralMesh))
      (bind (_isvalid _row _column) (Default|LocationtoTile (Variables|Default|GetGrid_Ref) (Math|Vector|MakeVector (.x (Transformation|GetWorldLocation _array_element)) (.y (Transformation|GetWorldLocation _array_element)) (.z (Transformation|GetWorldLocation _array_element)))))
      (bind _gridlocation (Default|TiletoGridLocation (Variables|Default|GetGrid_Ref) _row _column true))
      (bind _returnvalue (Game|SpawnActorfromClass "/Game/Blueprints/Combat/BP_CheckingVolume.BP_CheckingVolume_C" (Math|Transform|MakeTransform (Math|Conversions|ToVector(Vector2D) _gridlocation (.z (Transformation|GetWorldLocation _array_element))) "0, 0, 0" "1.000000,1.000000,1.000000") "Undefined" "MultiplyWithRoot" 0 0))
      (if (> (Utilities|Array|Length (Collision|GetOverlappingActors _returnvalue "/Game/Blueprints/AI/BP_BasicEnemy.BP_BasicEnemy_C" :!class /Script/Engine.Actor)) 0)
        (Default|UpdateHealthBar (.AsBP%20Basic%20Enemy (Utilities|Casting|CastToBP_BasicEnemy (Utilities|Array|Get(acopy) (Collision|GetOverlappingActors _returnvalue "/Game/Blueprints/AI/BP_BasicEnemy.BP_BasicEnemy_C" :!class /Script/Engine.Actor)))) true (Variables|Default|GetBarrelDamage)))
      (if (> (Utilities|Array|Length (Collision|GetOverlappingActors _returnvalue "/Game/TopDown/Blueprints/BP_TopDownCharacter.BP_TopDownCharacter_C" :!class /Script/Engine.Actor)) 0)
        (bind _asbp_top_down_character (Utilities|Casting|CastToBP_TopDownCharacter (Utilities|Array|Get(acopy) (Collision|GetOverlappingActors _returnvalue "/Game/TopDown/Blueprints/BP_TopDownCharacter.BP_TopDownCharacter_C" :!class /Script/Engine.Actor))))
        (Default|UpdateHealthBar _asbp_top_down_character 5e+01))
      (Actor|DestroyActor _returnvalue))
    (Actor|DestroyActor)))

(fn ConstructionScript)

(fn CreateMaterialInstance
  (params (Color :type Linear%20Color%20Structure) (Opacity :type Float%20%28double-precision%29))
  (bind _returnvalue (Rendering|Material|CreateDynamicMaterialInstance "/Game/Blueprints/Grid/M_Grid.M_Grid" "None" "None" :!class /Script/Engine.KismetMaterialLibrary))
  (Rendering|Material|SetVectorParameterValue _returnvalue "Color" Color :!class /Script/Engine.MaterialInstanceDynamic)
  (Rendering|Material|SetScalarParameterValue _returnvalue "Opacity" Opacity :!class /Script/Engine.MaterialInstanceDynamic)
  (return _returnvalue))