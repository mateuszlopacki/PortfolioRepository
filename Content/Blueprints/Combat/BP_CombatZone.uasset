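; Combat zone trigger that starts and ends turn-based grid combat when the player enters an area containing basic enemies.
; On entry it swaps the game mode's grid to its combat grid, updates enemy AI and broadcasts combat state to actors and widgets through I_Combat.
; CombatEndCheck restores the main grid once no enemies remain, otherwise it rebuilds the enemy list and rebroadcasts it with a bounds-checked turn index.
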(event Custom|EnteredCombatZone
  (if (> (Utilities|Array|Length (Collision|GetOverlappingActors (Variables|Default|GetCombatZone) "/Game/Blueprints/AI/BP_BasicEnemy.BP_BasicEnemy_C" :!class /Script/Engine.PrimitiveComponent)) 0)
    (bind _asbp_top_down_game_mode (Utilities|Casting|CastToBP_TopDownGameMode (Game|GetGameMode)))
    (bind _output_get (Variables|/Game/TopDown/Blueprints/BP_TopDownGameMode.BP_TopDownGameMode_C|SetGrids _asbp_top_down_game_mode (Variables|Default|GetCombatGrid)))
    (Rendering|SetActorHiddenInGame _output_get false)
    (for _array_element (Collision|GetOverlappingActors (Variables|Default|GetCombatZone) "/Game/Blueprints/AI/BP_BasicEnemy.BP_BasicEnemy_C" :!class /Script/Engine.PrimitiveComponent)
      (bind _asbp_basic_enemy (Utilities|Casting|CastToBP_BasicEnemy _array_element))
      (Utilities|Array|Add (Variables|Default|GetEnemiesArray) _asbp_basic_enemy)
      (bind _asaic_basic_enemy_controller (Utilities|Casting|CastToAIC_BasicEnemyController (AI|GetAIController _array_element)))
      (Default|UpdateCombatStatus _asaic_basic_enemy_controller))
    (bind _outactors (Actor|GetAllActorswithInterface "/Game/Interfaces/I_Combat.I_Combat_C"))
    (for _array_element_2 _outactors
      (Class|ICombat|UpdateCombatStatus(Message) _array_element_2 true false false)
      (Class|ICombat|UpdateEnemiesInsideCombat(Message) _array_element_2 (Variables|Default|GetEnemiesArray))
      (Class|ICombat|ChangeTurnIndex(Message) _array_element_2))
    (bind _foundwidgets (Class|WidgetBlueprintLibrary|GetAllWidgetswithInterface "/Game/Interfaces/I_Combat.I_Combat_C" false))
    (for _array_element_3 _foundwidgets
      (Class|ICombat|UpdateCombatStatus(Message) _array_element_3 true false false)
      (Class|ICombat|ChangeTurnIndex(Message) _array_element_3))
    (Utilities|Array|Clear (Variables|Default|GetEnemies))))

(event Custom|CombatEndCheck
  (bind _enemiesarray (Variables|Default|GetEnemiesArray))
  (bind _enemiesarray_2 (Variables|Default|GetEnemiesArray))
  (bind _currentturnindex (Variables|Default|GetCurrentTurnIndex))
  (bind _currentturnindex_2 (Variables|Default|GetCurrentTurnIndex))
  (bind _returnvalue (== _currentturnindex 0))
  (bind _returnvalue_2 (== _currentturnindex_2 0))
  (if (== (Utilities|Array|Length (Collision|GetOverlappingActors (Variables|Default|GetCombatZone) "/Game/Blueprints/AI/BP_BasicEnemy.BP_BasicEnemy_C" :!class /Script/Engine.PrimitiveComponent)) 0)
    (Rendering|SetActorHiddenInGame (Variables|Default|GetCombatGrid) true)
    (bind _returnvalue_3 (Actor|GetActorOfClass "/Game/Blueprints/Grid/BP_MainGrid.BP_MainGrid_C"))
    (bind _asbp_top_down_game_mode (Utilities|Casting|CastToBP_TopDownGameMode (Game|GetGameMode)))
    (Variables|/Game/TopDown/Blueprints/BP_TopDownGameMode.BP_TopDownGameMode_C|SetGrids _asbp_top_down_game_mode _returnvalue_3)
    (bind _outactors (Actor|GetAllActorswithInterface "/Game/Interfaces/I_Combat.I_Combat_C"))
    (for _array_element _outactors
      (Class|ICombat|UpdateCombatStatus(Message) _array_element false false false))
    (bind _foundwidgets (Class|WidgetBlueprintLibrary|GetAllWidgetswithInterface "/Game/Interfaces/I_Combat.I_Combat_C" false))
    (for _array_element_2 _foundwidgets
      (Class|ICombat|UpdateCombatStatus(Message) _array_element_2 false false false))
    (else
      (Utilities|Array|Clear (Variables|Default|GetEnemiesArray))
      (for _array_element_3 (Collision|GetOverlappingActors (Variables|Default|GetCombatZone) "/Game/Blueprints/AI/BP_BasicEnemy.BP_BasicEnemy_C" :!class /Script/Engine.PrimitiveComponent)
        (bind _asbp_basic_enemy (Utilities|Casting|CastToBP_BasicEnemy _array_element_3))
        (Utilities|Array|Add (Variables|Default|GetEnemiesArray) _asbp_basic_enemy))
      (bind _outactors_2 (Actor|GetAllActorswithInterface "/Game/Interfaces/I_Combat.I_Combat_C"))
      (for _array_element_4 _outactors_2
        (Class|ICombat|UpdateEnemiesInsideCombat(Message) _array_element_4 _enemiesarray_2)
        (if (> (Variables|Default|GetCurrentTurnIndex) (Utilities|Array|Length _enemiesarray_2))
          (if (not _returnvalue)
            (Class|ICombat|ChangeTurnIndex(Message) _array_element_4))
          (elif (not _returnvalue)
            (Class|ICombat|ChangeTurnIndex(Message) _array_element_4 (Variables|Default|GetCurrentTurnIndex)))))
      (bind _foundwidgets_2 (Class|WidgetBlueprintLibrary|GetAllWidgetswithInterface "/Game/Interfaces/I_Combat.I_Combat_C" false))
      (for _array_element_5 _foundwidgets_2
        (Class|ICombat|UpdateEnemiesInsideCombat(Message) _array_element_5 _enemiesarray)
        (if (> (Variables|Default|GetCurrentTurnIndex) (Utilities|Array|Length _enemiesarray))
          (if (not _returnvalue_2)
            (Class|ICombat|ChangeTurnIndex(Message) _array_element_5))
          (elif (not _returnvalue_2)
            (Class|ICombat|ChangeTurnIndex(Message) _array_element_5 (Variables|Default|GetCurrentTurnIndex))))))))

(event EventBeginPlay
  (bind _asbp_top_down_character (Utilities|Casting|CastToBP_TopDownCharacter (Game|GetPlayerCharacter 0)))
  (Variables|Default|SetPlayerCharacterRef _asbp_top_down_character)
  (bind _asbp_top_down_controller (Utilities|Casting|CastToBP_TopDownController (Game|GetPlayerController 0)))
  (Variables|Default|SetPlayerControllerRef _asbp_top_down_controller))

(event Collision|EventActorBeginOverlap
  (params (OtherActor :type Actor%20Object%20Reference))
  (Utilities|Casting|CastToBP_TopDownCharacter OtherActor)
  (CallFunction|EnteredCombatZone))

(event EventTick
  (params (DeltaSeconds :type Float%20%28single-precision%29)))

(event EventChangeTurnIndex
  (params (TurnIndex :type Integer))
  (Variables|Default|SetCurrentTurnIndex TurnIndex))

(fn ConstructionScript)