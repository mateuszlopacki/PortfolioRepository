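; Turn-based boss fight manager that runs a clock-themed countdown hazard once the player enters its trigger box.
; ChangeTurnIndex picks a random clock quadrant, turns the hands and marks a 3x3 grid area with procedural meshes.
; The digit display drops every other turn; at zero an explosion heavily damages an overlapping BP_BasicEnemy, or the cycle restarts if none is caught.
; Combat mode ending activates the linked portal.
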(event OnComponentBeginOverlap(Box)
  (params (OverlappedComponent :type Primitive%20Component%20Object%20Reference) (OtherActor :type Actor%20Object%20Reference) (OtherComp :type Primitive%20Component%20Object%20Reference) (OtherBodyIndex :type Integer) (bFromSweep :type Boolean) (SweepResult :type Hit%20Result%20Structure%20%28by%20ref%29))
  (Utilities|Casting|CastToBP_TopDownCharacter OtherActor)
  (Variables|Default|SetShouldRun? true))

(event Custom|SetDamageTilesinPlaces
  (bind _hoursid (Variables|Default|GetHoursID))
  (bind _placestospawnvolume (Variables|Default|GetPlacesToSpawnVolume))
  (bind _gridref (Variables|Default|GetGridRef))
  (bind _gridref_2 (Variables|Default|GetGridRef))
  (bind _gridref_3 (Variables|Default|GetGridRef))
  (bind _gridref_4 (Variables|Default|GetGridRef))
  (bind _gridref_5 (Variables|Default|GetGridRef))
  (bind _gridref_6 (Variables|Default|GetGridRef))
  (bind _gridref_7 (Variables|Default|GetGridRef))
  (bind _gridref_8 (Variables|Default|GetGridRef))
  (bind _gridref_9 (Variables|Default|GetGridRef))
  (bind _output (Utilities|Array|Get(acopy) _placestospawnvolume _hoursid))
  (bind _returnvalue (Transformation|GetActorLocation _output))
  (bind (_isvalid _row _column) (Default|LocationtoTile (Variables|Default|GetGridRef) (Math|Vector|MakeVector (.x _returnvalue) (.y _returnvalue) (.z (Transformation|GetActorLocation (Variables|Default|GetGridRef))))))
  (Utilities|FlowControl|Sequence
    (:then_0
      (bind _gridlocation (Default|TiletoGridLocation _gridref_2 _row _column false))
      (Transformation|SetWorldLocation (Variables|Default|GetProceduralMesh3) (Math|Conversions|ToVector(Vector2D) _gridlocation (+ (.z (Transformation|GetActorLocation _gridref_2)) -1.0)) false false))
    (:then_1
      (bind _gridlocation_2 (Default|TiletoGridLocation _gridref_3 _row (+ _column 1) false))
      (Transformation|SetWorldLocation (Variables|Default|GetProceduralMesh2) (Math|Conversions|ToVector(Vector2D) _gridlocation_2 (+ (.z (Transformation|GetActorLocation _gridref_3)) -1.0)) false false))
    (:then_2
      (bind _gridlocation_3 (Default|TiletoGridLocation _gridref_4 _row (+ _column -1) false))
      (Transformation|SetWorldLocation (Variables|Default|GetProceduralMesh1) (Math|Conversions|ToVector(Vector2D) _gridlocation_3 (+ (.z (Transformation|GetActorLocation _gridref_4)) -1.0)) false false))
    (:then_3
      (bind _gridlocation_4 (Default|TiletoGridLocation _gridref_7 (+ _row 1) (+ _column 0) false))
      (Transformation|SetWorldLocation (Variables|Default|GetProceduralMesh) (Math|Conversions|ToVector(Vector2D) _gridlocation_4 (+ (.z (Transformation|GetActorLocation _gridref_7)) -1.0)) false false))
    (:then_4
      (bind _gridlocation_5 (Default|TiletoGridLocation _gridref_8 (+ _row 1) (+ _column 1) false))
      (Transformation|SetWorldLocation (Variables|Default|GetProceduralMesh8) (Math|Conversions|ToVector(Vector2D) _gridlocation_5 (+ (.z (Transformation|GetActorLocation _gridref_8)) -1.0)) false false))
    (:then_5
      (bind _gridlocation_6 (Default|TiletoGridLocation _gridref_9 (+ _row 1) (+ _column -1) false))
      (Transformation|SetWorldLocation (Variables|Default|GetProceduralMesh7) (Math|Conversions|ToVector(Vector2D) _gridlocation_6 (+ (.z (Transformation|GetActorLocation _gridref_9)) -1.0)) false false))
    (:then_6
      (bind _gridlocation_7 (Default|TiletoGridLocation _gridref_5 (+ _row -1) (+ _column 0) false))
      (Transformation|SetWorldLocation (Variables|Default|GetProceduralMesh4) (Math|Conversions|ToVector(Vector2D) _gridlocation_7 (+ (.z (Transformation|GetActorLocation _gridref_5)) -1.0)) false false))
    (:then_7
      (bind _gridlocation_8 (Default|TiletoGridLocation _gridref_6 (+ _row -1) (+ _column 1) false))
      (Transformation|SetWorldLocation (Variables|Default|GetProceduralMesh6) (Math|Conversions|ToVector(Vector2D) _gridlocation_8 (+ (.z (Transformation|GetActorLocation _gridref_6)) -1.0)) false false))
    (:then_8
      (bind _gridlocation_9 (Default|TiletoGridLocation _gridref (+ _row -1) (+ _column -1) false))
      (Transformation|SetWorldLocation (Variables|Default|GetProceduralMesh5) (Math|Conversions|ToVector(Vector2D) _gridlocation_9 (+ (.z (Transformation|GetActorLocation _gridref)) -1.0)) false false)
      (Rendering|SetVisibility (Variables|Default|GetProceduralMesh6) true false))))

(event Custom|Display0
  (for _array_element (Variables|Default|GetNumbersMeshesArray)
    (Rendering|SetActorHiddenInGame _array_element false))
  (for _array_element_2 (Variables|Default|GetNumber0Array)
    (Rendering|SetActorHiddenInGame _array_element_2 true)))

(event Custom|Display1
  (for _array_element (Variables|Default|GetNumbersMeshesArray)
    (Rendering|SetActorHiddenInGame _array_element false))
  (for _array_element_2 (Variables|Default|GetNumber1Array)
    (Rendering|SetActorHiddenInGame _array_element_2 true)))

(event Custom|Display2
  (for _array_element (Variables|Default|GetNumbersMeshesArray)
    (Rendering|SetActorHiddenInGame _array_element false))
  (for _array_element_2 (Variables|Default|GetNumber2Array)
    (Rendering|SetActorHiddenInGame _array_element_2 true)))

(event Custom|Display3
  (for _array_element (Variables|Default|GetNumbersMeshesArray)
    (Rendering|SetActorHiddenInGame _array_element false))
  (for _array_element_2 (Variables|Default|GetNumber3Array)
    (Rendering|SetActorHiddenInGame _array_element_2 true)))

(event Custom|DisplayHours69
  (Transformation|SetActorRotation (Variables|Default|GetBigArrow) "0.000000,270.000000,0.000000")
  (Transformation|SetActorRotation (Variables|Default|GetSmallArrow) "0.000000,180.000000,0.000000"))

(event Custom|DisplayHours36
  (Transformation|SetActorRotation (Variables|Default|GetBigArrow) "0.000000,180.000000,0.000000")
  (Transformation|SetActorRotation (Variables|Default|GetSmallArrow) "0.000000,90.000000,0.000000"))

(event Custom|DisplayHours123
  (Transformation|SetActorRotation (Variables|Default|GetBigArrow) "0.000000,90.000000,0.000000")
  (Transformation|SetActorRotation (Variables|Default|GetSmallArrow)))

(event Custom|DisplayHours912
  (Transformation|SetActorRotation (Variables|Default|GetBigArrow))
  (Transformation|SetActorRotation (Variables|Default|GetSmallArrow) "0.000000,270.000000,0.000000"))

(event EventBeginPlay
  (bind _gridref (Variables|Default|GetGridRef))
  (bind _materialinstance (CallFunction|CreateMaterialInstance (Variables|Default|GetDamage%20Tiles%20Color) (Variables|Default|GetDamage%20Tiles%20Opacity)))
  (Variables|Default|SetDamageTilesMaterial _materialinstance)
  (Class|ProceduralMeshComponent|CreateMeshSectionLinearColor (Variables|Default|GetProceduralMesh6) 0 (Variables|/Game/Blueprints/Grid/BP_Grid.BP_Grid_C|GetSelection%20Vertices _gridref) (Variables|/Game/Blueprints/Grid/BP_Grid.BP_Grid_C|GetSelection%20Triangles _gridref) 0 0 0 0 0 0 0 false false)
  (Rendering|Material|SetMaterial (Variables|Default|GetProceduralMesh6) 0 (Variables|Default|GetDamageTilesMaterial))
  (Rendering|SetVisibility (Variables|Default|GetProceduralMesh6) false false))

(event Collision|EventActorBeginOverlap
  (params (OtherActor :type Actor%20Object%20Reference)))

(event EventTick
  (params (DeltaSeconds :type Float%20%28single-precision%29)))

(event EventChangeTurnIndex
  (params (TurnIndex :type Integer))
  (if (Variables|Default|GetShouldRun?)
    (Utilities|FlowControl|Delay 0.2)
    (Variables|Default|SetCounter (+ (Variables|Default|GetCounter) 1))
    (if (== (Variables|Default|GetCounter) 1)
      (CallFunction|Display3)
      (switch int (Math|Random|RandomInteger 3)
        (:0
          (Variables|Default|SetHoursID 0)
          (CallFunction|DisplayHours123))
        (:1
          (Variables|Default|SetHoursID 2)
          (CallFunction|DisplayHours69))
        (:2
          (Variables|Default|SetHoursID 2)
          (CallFunction|DisplayHours69))
        (:3
          (Variables|Default|SetHoursID 3)
          (CallFunction|DisplayHours912)))
      (CallFunction|SetDamageTilesinPlaces)
      (elif (== (Math|Integer|%(Integer) (Variables|Default|GetCounter) 2) 1)
        (Variables|Default|SetCounterForNumbers (+ (Variables|Default|GetCounterForNumbers) 1))
        (switch int (Variables|Default|GetCounterForNumbers)
          (:1
            (CallFunction|Display2))
          (:2
            (CallFunction|Display1))
          (:3
            (CallFunction|Display0)
            (Niagara|SpawnSystematLocation "/Game/FX/NS_BossBattleBoom.NS_BossBattleBoom" (Transformation|GetActorLocation (Utilities|Array|Get(acopy) (Variables|Default|GetPlacesToSpawnVolume) (Variables|Default|GetHoursID))))
            (bind _returnvalue (Game|SpawnActorfromClass "/Game/Blueprints/Combat/BP_CheckingVolume.BP_CheckingVolume_C" (Math|Transform|MakeTransform (Transformation|GetActorLocation (Utilities|Array|Get(acopy) (Variables|Default|GetPlacesToSpawnVolume) (Variables|Default|GetHoursID))) "0, 0, 0" "2.750000,2.750000,1.000000") "Undefined" "MultiplyWithRoot" 0 0))
            (if (> (Utilities|Array|Length (Collision|GetOverlappingActors _returnvalue "/Game/Blueprints/AI/BP_BasicEnemy.BP_BasicEnemy_C" :!class /Script/Engine.Actor)) 0)
              (Default|UpdateHealthBar (.AsBP%20Basic%20Enemy (Utilities|Casting|CastToBP_BasicEnemy (Utilities|Array|Get(acopy) (Collision|GetOverlappingActors _returnvalue "/Game/Blueprints/AI/BP_BasicEnemy.BP_BasicEnemy_C" :!class /Script/Engine.Actor)))) true 1500)
              (Actor|DestroyActor _returnvalue)
              (Rendering|SetVisibility (Variables|Default|GetProceduralMesh6) false false)
              (else
                (Actor|DestroyActor _returnvalue)
                (Utilities|FlowControl|Delay 2.0)
                (Variables|Default|SetCounterForNumbers 0)
                (switch int (Math|Random|RandomInteger 3)
                  (:0
                    (Variables|Default|SetHoursID 0)
                    (CallFunction|DisplayHours123))
                  (:1
                    (Variables|Default|SetHoursID 1)
                    (CallFunction|DisplayHours36))
                  (:2
                    (Variables|Default|SetHoursID 2)
                    (CallFunction|DisplayHours69))
                  (:3
                    (Variables|Default|SetHoursID 3)
                    (CallFunction|DisplayHours912)))
                (CallFunction|SetDamageTilesinPlaces)
                (CallFunction|Display3)))))))))

(event EventUpdateCombatStatus
  (params (IsCombatModeEnabled :type Boolean) (IsMovementSelected :type Boolean) (IsSkillSelected :type Boolean))
  (if (Variables|Default|GetShouldRun?)
    (if (not IsCombatModeEnabled)
      (Default|ActivatePortal (Variables|Default|GetPortalToActivate))
      (Rendering|SetVisibility (Variables|Default|GetProceduralMesh6) true false))))

(fn ConstructionScript)

(fn CreateMaterialInstance
  (params (Color :type Linear%20Color%20Structure) (Opacity :type Float%20%28double-precision%29))
  (bind _returnvalue (Rendering|Material|CreateDynamicMaterialInstance "/Game/Blueprints/Grid/M_Grid.M_Grid" "None" "None" :!class /Script/Engine.KismetMaterialLibrary))
  (Rendering|Material|SetVectorParameterValue _returnvalue "Color" Color :!class /Script/Engine.MaterialInstanceDynamic)
  (Rendering|Material|SetScalarParameterValue _returnvalue "Opacity" Opacity :!class /Script/Engine.MaterialInstanceDynamic)
  (return _returnvalue))