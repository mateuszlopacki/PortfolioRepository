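; BP_Spikes is a combat trap that pops up on turn changes to damage an enemy standing on it.
; When the turn index is 1 and the player character is in its combat zone, it teleports upward briefly, then returns.
; A temporary BP_CheckingVolume finds the first overlapping BP_BasicEnemy, whose UpdateHealthBar applies fixed damage.
; A looping timer handle guards against re-triggering, but is cleared only after a completed spike cycle.
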(event EventBeginPlay
  (Variables|Default|SetActorLocation (Transformation|GetActorLocation)))

(event Collision|EventActorBeginOverlap
  (params (OtherActor :type Actor%20Object%20Reference)))

(event EventTick
  (params (DeltaSeconds :type Float%20%28single-precision%29)))

(event EventChangeTurnIndex
  (params (TurnIndex :type Integer))
  (bind _actorlocation (Variables|Default|GetActorLocation))
  (bind _returnvalue (+ _actorlocation "0.000000,0.000000,50.000000"))
  (if (not (Utilities|Time|IsTimerActivebyHandle (Variables|Default|GetTimerHandle)))
    (bind _returnvalue_2 (Utilities|Time|SetTimerbyEvent 0 0.1 true))
    (Variables|Default|SetTimerHandle _returnvalue_2)
    (if (and (== TurnIndex 1) (> (Utilities|Array|Length (Collision|GetOverlappingActors (Variables|Default|GetCombatZoneRef) "/Game/TopDown/Blueprints/BP_TopDownCharacter.BP_TopDownCharacter_C" :!class /Script/Engine.Actor)) 0))
      (Transformation|SetActorLocation _returnvalue false true)
      (bind _returnvalue_3 (Game|SpawnActorfromClass "/Game/Blueprints/Combat/BP_CheckingVolume.BP_CheckingVolume_C" (Math|Transform|MakeTransform _returnvalue "0, 0, 0" "1.000000,1.000000,1.000000") "Undefined" "MultiplyWithRoot" 0 0))
      (if (> (Utilities|Array|Length (Collision|GetOverlappingActors _returnvalue_3 "/Game/Blueprints/AI/BP_BasicEnemy.BP_BasicEnemy_C" :!class /Script/Engine.Actor)) 0)
        (bind _asbp_basic_enemy (Utilities|Casting|CastToBP_BasicEnemy (Utilities|Array|Get(acopy) (Collision|GetOverlappingActors _returnvalue_3 "/Game/Blueprints/AI/BP_BasicEnemy.BP_BasicEnemy_C" :!class /Script/Engine.Actor)))
          (:then
            (Actor|DestroyActor _returnvalue_3)
            (Utilities|IsValid _asbp_basic_enemy
              (:Is%20Valid
                (Default|UpdateHealthBar _asbp_basic_enemy true 30))
              (:Is%20Not%20Valid
                _)))
          (:CastFailed
            (Actor|DestroyActor _returnvalue_3 :!label _label)))
        (else
          (goto _label)))
      (Utilities|FlowControl|Delay 0.5)
      (Transformation|SetActorLocation (Variables|Default|GetActorLocation) false true)
      (Utilities|Time|ClearandInvalidateTimerbyHandle (Variables|Default|GetTimerHandle)))))

(fn ConstructionScript)