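; BP_Credits is a trigger actor that shows a text popup, presumably the credits, once its referenced Portal is activated.
; When BP_TopDownCharacter overlaps it with the portal active, a DoOnce lets the sequence run a single time.
; It stops the character's movement, writes its DisplayedText into the CombatHUD popup and shows it, then makes the player controller ignore move input.
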(event EventBeginPlay)

(event EventTick
  (params (DeltaSeconds :type Float%20%28single-precision%29))
  (|CallParentFunction DeltaSeconds) ; This node is disabled and will not be called.\nDrag off pins to build functionality.
)

(event Collision|EventActorBeginOverlap
  (params (OtherActor :type Actor%20Object%20Reference))
  (bind _asbp_top_down_character (Utilities|Casting|CastToBP_TopDownCharacter OtherActor))
  (if (Variables|/Game/Blueprints/EnvironmentActors/BP_Portal.BP_Portal_C|GetActivated? (Variables|Default|GetPortal))
    (Utilities|FlowControl|DoOnce false
      (:Completed
        (AI|Navigation|StopMovement (Pawn|GetController _asbp_top_down_character))
        (bind _ascombat_hud (Utilities|Casting|CastToCombatHUD (HUD|GetHUD (Game|GetPlayerController 0))))
        (Variables|/Game/HUDs/WB_TextPopup.WB_TextPopup_C|SetDisplayedText (Variables|/Game/HUDs/CombatHUD.CombatHUD_C|GetTextPopup_Ref _ascombat_hud) (Variables|Default|GetDisplayed%20Text))
        (Widget|SetVisibility (Variables|/Game/HUDs/CombatHUD.CombatHUD_C|GetTextPopup_Ref _ascombat_hud) "HitTestInvisible")
        (bind _asbp_top_down_controller (Utilities|Casting|CastToBP_TopDownController (Game|GetPlayerController 0)))
        (Input|SetIgnoreMoveInput _asbp_top_down_controller true)))))

(fn ConstructionScript
  (|CallParentFunction))