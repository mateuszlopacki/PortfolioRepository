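; BP_ShallowWater is an environment actor that turns shallow water to ice when hit by a matching skill.
; On overlap with a BP_CheckingVolume, it compares the grid's SkillIDToCast against its own SkillID.
; On a match it destroys every valid actor in its Actor array and swaps the material on its three static meshes to MI_Ice.
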(event EventBeginPlay
  (|CallParentFunction) ; This node is disabled and will not be called.\nDrag off pins to build functionality.
)

(event EventTick
  (params (DeltaSeconds :type Float%20%28single-precision%29))
  (|CallParentFunction DeltaSeconds) ; This node is disabled and will not be called.\nDrag off pins to build functionality.
)

(event Collision|EventActorBeginOverlap
  (params (OtherActor :type Actor%20Object%20Reference))
  (Utilities|Casting|CastToBP_CheckingVolume OtherActor)
  (if (== (Variables|/Game/Blueprints/Grid/BP_Grid.BP_Grid_C|GetSkill_ID_To_Cast (Variables|Default|GetMainGridRef)) (Variables|Default|GetSkill_ID))
    (for _array_element (Variables|Default|GetActor)
      (Utilities|IsValid _array_element
        (:Is%20Valid
          (Actor|DestroyActor _array_element))))
    (Rendering|Material|SetMaterial (Variables|Default|GetStaticMesh) 0 "/Game/Materials/MI_Ice.MI_Ice")))

(fn ConstructionScript
  (|CallParentFunction))