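; Debug grid pathfinder actor that, on pressing Q, steps greedily from its tile toward the player character's tile.
; Each step gathers four orthogonal neighbors, filters blocked ones with temporary overlap volumes, and spawns green markers on free tiles.
; The free tile nearest the target by 2D distance turns lavender and becomes the current tile.
; Delays and printouts pace the loop until it reaches the target, without backtracking.
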(event EventBeginPlay
  (Input|EnableInput (Game|GetPlayerController 0)))

(event Collision|EventActorBeginOverlap
  (params (OtherActor :type Actor%20Object%20Reference)))

(event EventTick
  (params (DeltaSeconds :type Float%20%28single-precision%29)))

(event Input|KeyboardEvents|Q
  (params (Key :type Key%20Structure))
  (:Pressed
    (Utilities|IsValid (Variables|Default|GetGrid)
      (:Is%20Valid
        _)
      (:Is%20Not%20Valid
        (bind _asbp_top_down_game_mode (Utilities|Casting|CastToBP_TopDownGameMode (Game|GetGameMode)))
        (Variables|Default|SetGrid (Default|GetGrid _asbp_top_down_game_mode true))))
    (bind (_isvalid _row _column) (Default|LocationtoTile (Variables|Default|GetGrid) (Transformation|GetActorLocation)))
    (bind _gridlocation (Default|TiletoGridLocation (Variables|Default|GetGrid) _row _column true))
    (Variables|Default|SetCenterTileLocation (Math|Conversions|ToVector(Vector2D) _gridlocation (.z (Transformation|GetActorLocation))))
    (Variables|Default|SetPathfinderRow _row)
    (Variables|Default|SetPathfinderColumn _column)
    (bind _asbp_top_down_character (Utilities|Casting|CastToBP_TopDownCharacter (Game|GetPlayerCharacter 0)))
    (bind (_isvalid_2 _row_2 _column_2) (Default|LocationtoTile (Variables|Default|GetGrid) (Transformation|GetActorLocation _asbp_top_down_character)))
    (bind _output_get (Variables|Default|SetPlayerRow _row_2))
    (bind _output_get_2 (Variables|Default|SetPlayerColumn _column_2))
    (bind _gridlocation_2 (Default|TiletoGridLocation (Variables|Default|GetGrid) (Variables|Default|GetPlayerRow) (Variables|Default|GetPlayerColumn) true))
    (Variables|Default|SetPlayerTileGrid%20Location _gridlocation_2)
    (Development|PrintString "Player Row Is")
    (Development|PrintString (Utilities|String|ToString(Integer) _output_get))
    (Development|PrintString "Player Column Is")
    (Development|PrintString (Utilities|String|ToString(Integer) _output_get_2))
    (if (and (== (Variables|Default|GetPathfinderRow) (Variables|Default|GetPlayerRow)) (== (Variables|Default|GetPlayerColumn) (Variables|Default|GetPathfinderColumn))) :!label _label
      (Development|PrintString "Contragts, process complete")
      (else
        (bind _neighbortiles (CallFunction|CheckNeighborTiles (Variables|Default|GetPathfinderRow) (Variables|Default|GetPathfinderColumn)))
        (Utilities|FlowControl|Delay 1.0)
        (bind _validtiles (CallFunction|AnalyzeNeighborTiles _neighbortiles))
        (Utilities|FlowControl|Delay 1.0)
        (bind _newcentertile (CallFunction|PickTileClosesttoTarget _validtiles))
        (bind _output_get_3 (Variables|Default|SetCenterTileLocation (Math|Conversions|ToVector(Vector2D) _newcentertile (.z (Transformation|GetActorLocation)))))
        (bind (_isvalid_3 _row_3 _column_3) (Default|LocationtoTile (Variables|Default|GetGrid) _output_get_3))
        (Variables|Default|SetPathfinderRow _row_3)
        (Variables|Default|SetPathfinderColumn _column_3)
        (Utilities|FlowControl|Delay 1.0)
        (Development|PrintString "Current Row is")
        (Development|PrintString (Utilities|String|ToString(Integer) (Variables|Default|GetPathfinderRow)))
        (Development|PrintString "Current Column is")
        (Development|PrintString (Utilities|String|ToString(Integer) (Variables|Default|GetPathfinderColumn)))
        (goto _label)))))

(fn ConstructionScript)

(fn CheckNeighborTiles
  (params (Row :type Integer) (Column :type Integer))
  (Utilities|FlowControl|Sequence
    (:then_0
      (bind _gridlocation (Default|TiletoGridLocation (Variables|Default|GetGrid) (+ Row -1) Column true))
      (Utilities|Array|Add (LocalVariables|GetNeighborTilesArray) _gridlocation))
    (:then_1
      (bind _gridlocation_2 (Default|TiletoGridLocation (Variables|Default|GetGrid) (+ Row 1) Column true))
      (Utilities|Array|Add (LocalVariables|GetNeighborTilesArray) _gridlocation_2))
    (:then_2
      (bind _gridlocation_3 (Default|TiletoGridLocation (Variables|Default|GetGrid) Row (+ Column 1) true))
      (Utilities|Array|Add (LocalVariables|GetNeighborTilesArray) _gridlocation_3))
    (:then_3
      (bind _gridlocation_4 (Default|TiletoGridLocation (Variables|Default|GetGrid) Row (+ Column -1) true))
      (Utilities|Array|Add (LocalVariables|GetNeighborTilesArray) _gridlocation_4)
      (return (LocalVariables|GetNeighborTilesArray)))))

(fn AnalyzeNeighborTiles
  (params (TilesToAnalyze :type Array%20of%20Vector%202D%20Structures))
  (Utilities|Array|Clear (LocalVariables|GetValidTiles_Local))
  (for _array_element TilesToAnalyze
    (bind _returnvalue (Game|SpawnActorfromClass "/Game/Blueprints/Combat/BP_CheckingVolume.BP_CheckingVolume_C" (Math|Transform|MakeTransform (Math|Conversions|ToVector(Vector2D) _array_element (.z (Transformation|GetActorLocation))) "0, 0, 0" "1.000000,1.000000,1.000000") "Undefined" "MultiplyWithRoot" 0 0))
    (if (> (Utilities|Array|Length (Collision|GetOverlappingActors _returnvalue 0 :!class /Script/Engine.Actor)) 1)
      _
      (else
        (bind _returnvalue_2 (Game|SpawnActorfromClass "/Game/Blueprints/Grid/BP_PathfinderPath.BP_PathfinderPath_C" (Math|Transform|MakeTransform (Math|Conversions|ToVector(Vector2D) _array_element (.z (Transformation|GetActorLocation))) "0, 0, 0" "1.000000,1.000000,1.000000") "Undefined" "MultiplyWithRoot" 0 0))
        (Rendering|Material|SetMaterial (Variables|/Game/Blueprints/Grid/BP_PathfinderPath.BP_PathfinderPath_C|GetSphere _returnvalue_2) 0 "/Game/Materials/MI_BasicColor_Green.MI_BasicColor_Green")
        (Utilities|Array|Add (LocalVariables|GetValidTiles_Local) _array_element)))
    (Actor|DestroyActor _returnvalue))
  (return (LocalVariables|GetValidTiles_Local)))

(fn PickTileClosesttoTarget
  (params (TilesToChooseFrom :type Array%20of%20Vector%202D%20Structures))
  (bind _distancesarray (LocalVariables|GetDistancesArray))
  (bind (_indexofminvalue _minvalue) (Math|Float|MinOfFloatArray _distancesarray))
  (bind _output (Utilities|Array|Get(acopy) TilesToChooseFrom _indexofminvalue))
  (Utilities|Array|Clear (LocalVariables|GetDistancesArray))
  (for _array_element TilesToChooseFrom
    (Utilities|Array|Add (LocalVariables|GetDistancesArray) (Math|Float|Absolute(Float) (Math|Vector|Distance2D(Vector) _array_element (Variables|Default|GetPlayerTileGrid%20Location)))))
  (Development|PrintString "Distance is")
  (Development|PrintString (Utilities|String|ToString(Float) _minvalue))
  (bind _returnvalue (Game|SpawnActorfromClass "/Game/Blueprints/Combat/BP_CheckingVolume.BP_CheckingVolume_C" (Math|Transform|MakeTransform (Math|Conversions|ToVector(Vector2D) _output (.z (Variables|Default|GetCenterTileLocation))) "0, 0, 0" "1.000000,1.000000,1.000000") "Undefined" "MultiplyWithRoot" 0 0))
  (bind _asbp_pathfinder_path (Utilities|Casting|CastToBP_PathfinderPath (Utilities|Array|Get(acopy) (Collision|GetOverlappingActors _returnvalue "/Game/Blueprints/Grid/BP_PathfinderPath.BP_PathfinderPath_C" :!class /Script/Engine.Actor))))
  (Rendering|Material|SetMaterial (Variables|/Game/Blueprints/Grid/BP_PathfinderPath.BP_PathfinderPath_C|GetSphere _asbp_pathfinder_path) 0 "/Game/Materials/MI_BasicColor_Lavender.MI_BasicColor_Lavender")
  (return _output))